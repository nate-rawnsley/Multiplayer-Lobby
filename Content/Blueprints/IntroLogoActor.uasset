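; Intro logo actor that animates the logo into place on the cube menu, then hands off to it.
; After a short delay, Tick slides it forward with a sine in-out lerp to follow the camera, then bounce-eases location and scale onto the menu.
; Once settled, it snaps to the final transform, tells the CubeMenu actor to show its own logo, and destroys itself a second later.
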(event `self.ReceiveBeginPlay`
  ;[1 1 1] The logo moves after 4 seconds, to follow the camera.
  (`KismetSystemLibrary.Delay` 4.0)
  (set `self.Move` true))

(event `self.ReceiveTick`
  (params (DeltaSeconds :type "Float (single-precision)"))
  (bind _lerptime (`self.LerpTime`))
  (if (`self.Move`)
    (`self.BeginningMove` DeltaSeconds)
    (elif (`self.BounceToUI`)
      (bind _returnvalue (`BlueprintEasingLibrary.EaseOutBounce` _lerptime))
      ;[1 1 1] Bounces onto the cube menu through lerping.
      (`self.K2_SetActorLocation` (`KismetMathLibrary.VLerp` (950.0 -20.0 65.0) (969.0 -20.0 45.0) _returnvalue))
      (`self.SetActorScale3D` (`KismetMathLibrary.VLerp` (0.25 0.25 0.25) (0.1 0.1 0.1) _returnvalue))
      (bind _output_get (set `self.LerpTime` (+ _lerptime DeltaSeconds)))
      (if (>= _output_get 1.0)
        (set `self.BounceToUI` false)
        ;[1 1 1] Eclipses the logo on the UI, and then sets it to visible.
        (`self.K2_SetActorLocation` (969.0 -20.0 45.0))
        (`self.SetActorScale3D` (0.1 0.1 0.1))
        (bind _returnvalue_2 (`GameplayStatics.GetActorOfClass` "/Game/Blueprints/CubeMenu.CubeMenu_C"))
        (`/Game/Blueprints/CubeMenu.ShowLogo` _returnvalue_2)
        ;[1 1 1] Destroys self once the logo is settled.
        (`KismetSystemLibrary.Delay` 1.0)
        (`self.K2_DestroyActor`)))))

(fn `BeginningMove`
  (params (DeltaTime :type "Float (double-precision)"))
  (bind _returnvalue (+ (`self.LerpTime`) (* DeltaTime 0.5)))
  (if (>= _returnvalue 1.0)
    (set `self.LerpTime` 0.0)
    ;[1 1 1] Once the loop is over, starts to lerp scale and position to the cube menu.
    (`self.K2_SetActorLocation` (950.0 -20.0 65.0))
    (set `self.Move` false)
    (set `self.BounceToUI` true)
    (else
      (bind _output_get (set `self.LerpTime` _returnvalue))
      (bind _returnvalue_2 (`BlueprintEasingLibrary.SineInOut` _output_get))
      (`self.K2_SetActorLocation` (`KismetMathLibrary.VLerp` (550.0 -20.0 65.0) (950.0 -20.0 65.0) _returnvalue_2)))))

(fn `UserConstructionScript`)