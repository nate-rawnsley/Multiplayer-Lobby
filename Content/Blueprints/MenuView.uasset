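; MenuView is an actor that glides between preset menu viewpoints, moving to the first one four seconds after play begins.
; ChangeLocation stores the current and chosen position plus yaw as Vector4s, starts the move and plays audio.
; Tick blends both with sine in-out easing, snaps to the target on completion and resets the move speed.
; The whoosh sound is assigned only after the first move starts, keeping startup silent.
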(event `self.ReceiveBeginPlay`
  ;[1 1 1] Only sets sound after the first movement, to prevent unnecesary sounds at the start.
  (`KismetSystemLibrary.Delay` 4.0)
  (`self.ChangeLocation` 0)
  (`AudioComponent.SetSound` (`self.Audio`) "/Game/Sounds/whoosh-gaming-jump-243507.whoosh-gaming-jump-243507"))

(event `self.ReceiveTick`
  (params (DeltaSeconds :type "Float (single-precision)"))
  (bind _movetargets (`self.MoveTargets`))
  (bind (_output_x _output_y _output_z _output_w) (`KismetMathLibrary.BreakVector4` (`|GetArrayItem` _movetargets 1)))
  (bind (_output_x_2 _output_y_2 _output_z_2 _output_w_2) (`KismetMathLibrary.BreakVector4` (`|GetArrayItem` _movetargets)))
  (bind (_output_x_3 _output_y_3 _output_z_3 _output_w_3) (`KismetMathLibrary.BreakVector4` (`|GetArrayItem` (`self.MoveTargets`) 1)))
  (bind _returnvalue (+ (`self.MovingTime`) (* (`self.MoveSpeed`) DeltaSeconds)))
  (if (`self.Moving`)
    (if (>= _returnvalue 1.0)
      (set `self.MovingTime` 0.0)
      (`self.K2_SetActorLocationAndRotation` (`KismetMathLibrary.MakeVector` _output_x_3 _output_y_3 _output_z_3) (`KismetMathLibrary.MakeRotator` 0.0 0.0 _output_w_3))
      ;[1 1 1] Resets move speed after the movement is done, in case it was changed before
      (set `self.Moving` false)
      (set `self.MoveSpeed` 1.0)
      (else
        ;[1 1 1] Lerps both the position and yaw together, with the same easing.
        (bind _output_get (set `self.MovingTime` _returnvalue))
        (bind _returnvalue_2 (`BlueprintEasingLibrary.SineInOut` _output_get))
        (`self.K2_SetActorLocationAndRotation` (`KismetMathLibrary.VLerp` (`KismetMathLibrary.MakeVector` _output_x_2 _output_y_2 _output_z_2) (`KismetMathLibrary.MakeVector` _output_x _output_y _output_z) _returnvalue_2) (`KismetMathLibrary.MakeRotator` 0.0 0.0 (`KismetMathLibrary.Lerp` _output_w_2 _output_w _returnvalue_2)))))))

(fn `ChangeLocation`
  (params (Index :type Integer))
  (bind (_returnvalue_x _returnvalue_y _returnvalue_z) (`KismetMathLibrary.BreakVector` (`self.K2_GetActorLocation`)))
  (bind (_returnvalue_roll _returnvalue_pitch _returnvalue_yaw) (`KismetMathLibrary.BreakRotator` (`self.K2_GetActorRotation`)))
  (bind _movetargets (`self.MoveTargets`))
  (`KismetArrayLibrary.Array_Set` _movetargets 0 (`KismetMathLibrary.MakeVector4` _returnvalue_x _returnvalue_y _returnvalue_z _returnvalue_yaw))
  (`KismetArrayLibrary.Array_Set` _movetargets 1 (`|GetArrayItem` (`self.Locations`) Index))
  (set `self.Moving` true)
  (`AudioComponent.Play` (`self.Audio`) 0.0))

(fn `UserConstructionScript`)