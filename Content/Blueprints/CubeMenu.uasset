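; Main menu cube actor whose faces host UI widgets, with functions to reveal the main logo and refresh every face's text.
; After a short delay, Tick raises and scales it into place with circular easing.
; RotateToFace starts a sine-eased turn to a face, ignoring calls mid-motion, and plays that face's sound or a back chord.
; Each turn randomizes which level spotlights are lit, fading their intensities alongside the rotation.
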(event `self.ReceiveBeginPlay`
  (set `PlayerController.bShowMouseCursor` true (`GameplayStatics.GetPlayerControllerFromID` 0))
  (bind _outactors (`GameplayStatics.GetAllActorsOfClass` "/Script/Engine.SpotLight"))
  (set `self.Spotlights` _outactors)
  ;[1 1 1] Start moving after 3 seconds
  (`KismetSystemLibrary.Delay` 3.0)
  (set `self.InPosition` false))

(event `self.ReceiveTick`
  (params (DeltaSeconds :type "Float (single-precision)"))
  (bind _currentrotationvals (`self.CurrentRotationVals`))
  (bind _lerptime (`self.LerpTime`))
  (bind _output (`|GetArrayItem` _currentrotationvals 1))
  (bind _returnvalue (+ DeltaSeconds _lerptime))
  ;[1 1 1] Lerping between cube faces
  (if (`self.Rotating`)
    (bind _returnvalue_2 (`BlueprintEasingLibrary.SineInOut` (`self.LerpTime`)))
    ;[1 1 1] Sets values to positive for more consistent rotation
    (bind _returnvalue_3 (`BlueprintEasingLibrary.PositiveRotator` (`|GetArrayItem` _currentrotationvals)))
    (bind _returnvalue_4 (`BlueprintEasingLibrary.PositiveRotator` _output))
    (`self.K2_SetActorRotation` (`KismetMathLibrary.RLerp` _returnvalue_3 _returnvalue_4 _returnvalue_2))
    (for (_array_element _array_index) (`self.Spotlights`)
      ;[1 1 1] Lerps the intensity of every light
      (`self.CheckLight` (`SpotLight.SpotLightComponent` _array_element) _array_index DeltaSeconds))
    (if (>= _returnvalue 1.0)
      (set `self.Rotating` false)
      (set `self.LerpTime` 0.0)
      (`self.K2_SetActorRotation` _output)
      (`self.ResetLightVals`)
      (else
        (set `self.LerpTime` _returnvalue)))
    (else
      ;[1 1 1] Scaling and moving at the beginning of the game
      (if (not (`self.InPosition`))
        (bind _returnvalue_5 (`BlueprintEasingLibrary.EaseOutCirc` (`self.LerpTime`)))
        (`self.K2_SetActorLocation` (`KismetMathLibrary.VLerp` (1020.0 -20.0 -146.0) (1020.0 -20.0 20.0) _returnvalue_5))
        (`self.SetActorScale3D` (`KismetMathLibrary.VLerp` (0.0 0.0 0.0) (1.0 1.0 1.0) _returnvalue_5))
        (bind _output_get (set `self.LerpTime` (+ (* DeltaSeconds 0.5) _lerptime)))
        (if (>= _output_get 1.0)
          (set `self.InPosition` true)
          (`self.K2_SetActorLocation` (1020.0 -20.0 20.0))
          (`self.SetActorScale3D` (1.0 1.0 1.0))
          (set `self.LerpTime` 0.0))))))

(fn `ChangeWidgetText`
  (bind _asmain_face (cast `/Game/Blueprints/UI/MainFace` (`WidgetComponent.GetWidget` (`self.Main Face`))))
  (`/Game/Blueprints/UI/MainFace.SetAllText` _asmain_face)
  (bind _asoptions_face (cast `/Game/Blueprints/UI/OptionsFace` (`WidgetComponent.GetWidget` (`self.Settings Face`))))
  (`/Game/Blueprints/UI/OptionsFace.SetAllText` _asoptions_face)
  (bind _asquit_face (cast `/Game/Blueprints/UI/QuitFace` (`WidgetComponent.GetWidget` (`self.Quit Face`))))
  (`/Game/Blueprints/UI/QuitFace.SetAllText` _asquit_face)
  (bind _asselection_face (cast `/Game/Blueprints/UI/SelectionFace` (`WidgetComponent.GetWidget` (`self.Select Face`))))
  (`/Game/Blueprints/UI/SelectionFace.SetAllText` _asselection_face)
  (bind _asplay_face (cast `/Game/Blueprints/UI/PlayFace` (`WidgetComponent.GetWidget` (`self.Play Face`))))
  (`/Game/Blueprints/UI/PlayFace.SetAllText` _asplay_face)
  (bind _ashost_face (cast `/Game/Blueprints/UI/HostFace` (`WidgetComponent.GetWidget` (`self.Host Face`))))
  (`/Game/Blueprints/UI/HostFace.SetAllText` _ashost_face))

(fn `CheckLight`
  (params (Light :type "SpotLightComponent Object Reference") (Index :type Integer) (Increment :type "Float (double-precision)"))
  (locals (LocalValue :type "Float (double-precision)") (LocalBool :type Boolean))
  (bind _returnvalue (* Increment 10.0))
  (bind _returnvalue_2 (+ (`local.LocalValue`) _returnvalue))
  (bind _returnvalue_3 (- (`local.LocalValue`) _returnvalue))
  ;[1 1 1] Lerps the intensity of a light.
  (set `local.LocalBool` (`|GetArrayItem` (`self.LightsOn`) Index))
  (set `local.LocalValue` (`|GetArrayItem` (`self.LightValues`) Index))
  (if (and (`local.LocalBool`) (< (`local.LocalValue`) 10.0))
    (`LightComponent.SetIntensity` (`local.Light`) _returnvalue_2)
    (`KismetArrayLibrary.Array_Set` (`self.LightValues`) (`local.Index`) _returnvalue_2)
    (elif (and (not (`local.LocalBool`)) (> (`local.LocalValue`) 0.0))
      (`LightComponent.SetIntensity` (`local.Light`) _returnvalue_3)
      (`KismetArrayLibrary.Array_Set` (`self.LightValues`) (`local.Index`) _returnvalue_3))))

(fn `RandomiseSpotlights`
  (bind _returnvalue (`KismetMathLibrary.RandomBool`))
  (bind _lightson (`self.LightsOn`))
  ;[1 1 1] Sets a random boolean for whether each light should be on.
  (for (_ _array_index) (`self.Spotlights`)
    (`KismetArrayLibrary.Array_Set` (`self.LightsOn`) _array_index _returnvalue)
    (if _returnvalue
      _))
  ;[1 1 1] If no lights are on, sets a random light to true.
  (if (not (`KismetArrayLibrary.Array_Contains` _lightson true))
    (`KismetArrayLibrary.Array_Set` _lightson (`KismetMathLibrary.RandomIntegerInRange` 0 2) true)))

(fn `ResetLightVals`
  (bind _lightvalues (`self.LightValues`))
  ;[1 1 1] At the end of a lerp, it checks whether each light should be on and ensures they are set to the correct values.
  (for (_ _array_index) (`self.LightValues`)
    (if (`|GetArrayItem` (`self.LightsOn`) _array_index)
      (`KismetArrayLibrary.Array_Set` _lightvalues _array_index 10.0)
      (bind _spotlightcomponent (`SpotLight.SpotLightComponent` (`|GetArrayItem` (`self.Spotlights`) _array_index)))
      (`LightComponent.SetIntensity` _spotlightcomponent 10.0)
      (else
        (`KismetArrayLibrary.Array_Set` _lightvalues _array_index)
        (`LightComponent.SetIntensity` _spotlightcomponent 0.0)))))

(fn `RotateToFace`
  (params (FaceIndex :type Integer) (BackSound :type Boolean))
  (bind _returnvalue (`self.K2_GetActorRotation`))
  (bind _currentrotationvals (`self.CurrentRotationVals`))
  (bind _audio (`self.Audio`))
  (bind _output (`|GetArrayItem` (`self.RotationValues`) FaceIndex))
  (if (not (or (or (not (`self.InPosition`)) (`self.Rotating`)) (== _returnvalue _output)))
    ;[1 1 1] Starts lerping in Event Tick
    (set `self.Rotating` true)
    ;[1 1 1] Sets the current rotation to the start and the target rotation to the end.
    (`KismetArrayLibrary.Array_Set` _currentrotationvals 0 _returnvalue)
    (`KismetArrayLibrary.Array_Set` _currentrotationvals 1 _output)
    ;[1 1 1] Randomises which spotlights are on
    (`self.RandomiseSpotlights`)
    ;[1 1 1] Plays a sound - either the predetermined sound for the target face, or the generic 'back' sound as specified when the function is called.
    (if (`local.BackSound`)
      (`AudioComponent.SetSound` _audio "/Game/Sounds/backChord.backChord")
      (else
        (`AudioComponent.SetSound` _audio (`|GetArrayItem` (`self.AudioClips`) (- (`local.FaceIndex`) 1)))))
    (`AudioComponent.Play` _audio 0.0)))

(fn `ShowLogo`
  ;[1 1 1] Called from IntroLogoActor, makes the logo and button on the main face appear.
  (bind _asmain_face (cast `/Game/Blueprints/UI/MainFace` (`WidgetComponent.GetWidget` (`self.Main Face`))))
  (`/Game/Blueprints/UI/MainFace.RevealLogo` _asmain_face))

(fn `UserConstructionScript`)