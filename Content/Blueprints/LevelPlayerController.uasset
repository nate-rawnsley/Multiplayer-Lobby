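; Player controller for session-based multiplayer levels that owns the level HUD and pause menu and handles leaving the session.
; BeginPlay creates both widgets for controller ID 0, then calls OtherJoin on every other controller in the GameState PlayerArray to show the join text.
; Pressing P reveals the pause menu and mouse cursor.
; EndPlay destroys the session and opens MainMenu on success, covering kicks and host departure.
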(event `self.ReceiveBeginPlay`
  (bind _returnvalue (`GameplayStatics.GetPlayerControllerFromID` 0))
  ;[1 1 1] Adds UI for both the pause menu and the text when a player joins at the start, to become visible later.
  (bind _returnvalue_2 (`|CreateWidget` "/Game/Blueprints/UI/LevelUI.LevelUI_C" _returnvalue))
  (bind _output_get (set `self.LevelUI` _returnvalue_2))
  (`UserWidget.AddToViewport` _output_get 0)
  (bind _returnvalue_3 (`|CreateWidget` "/Game/Blueprints/UI/PauseUI.PauseUI_C" _returnvalue))
  (bind _output_get_2 (set `self.PauseUI` _returnvalue_3))
  (`UserWidget.AddToViewport` _output_get_2 0)
  (set `Widget.Visibility` "Hidden" _output_get_2)
  ;[1 1 1] Makes the player join text appear on all players currently in the scene.
  (for _array_element (`GameStateBase.PlayerArray` (`GameplayStatics.GetGameState`))
    (bind _returnvalue_4 (`PlayerState.GetPlayerController` _array_element))
    (if (!= _returnvalue_4 (`GameplayStatics.GetPlayerControllerFromID` 0))
      (bind _aslevel_player_controller (cast `/Game/Blueprints/LevelPlayerController` _returnvalue_4))
      (`self.OtherJoin` _aslevel_player_controller))))

(event `Key|P`
  (params (Key :type "Key Structure"))
  ;[1 1 1] Shows pause menu when P is pressed.
  (:`Pressed`
    (`Widget.SetVisibility` (`self.PauseUI`) "Visible")
    (set `PlayerController.bShowMouseCursor` true (`GameplayStatics.GetPlayerControllerFromID` 0))))

(event `OtherJoin`
  (`/Game/Blueprints/UI/LevelUI.DisplayJoin` (`self.LevelUI`)))

(event `self.ReceiveEndPlay`
  (params (EndPlayReason :type "EEndPlayReason Enum" :default "Destroyed"))
  ;[1 1 1] Ensures the player properly leaves the session even when kicked (eg. host leaves game)
  (`DestroySessionCallbackProxy.DestroySession` self
    (:`OnSuccess`
      (`GameplayStatics.OpenLevel` "MainMenu"))))

(fn `UserConstructionScript`)