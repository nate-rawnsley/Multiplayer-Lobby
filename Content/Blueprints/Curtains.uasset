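; Curtain actor that slides two curtain components apart to open and back together to close.
; While the Opening or Closing flag is set, Tick advances a normalized position value, faster when opening, clamps it at either end and clears both flags.
; A sine in-out ease maps that value to mirrored relative X offsets, and the persistent value lets the direction reverse mid-animation.
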(event `self.ReceiveTick`
  (params (DeltaSeconds :type "Float (single-precision)"))
  (bind _opening (`self.Opening`))
  (bind _returnvalue (+ (* DeltaSeconds (select `bool` _opening :`false` -0.25 :`true` 0.5)) (`self.LocationVal`)))
  (if (or _opening (`self.Closing`))
    (set `self.LocationVal` _returnvalue)
    ;[1 1 1] If the value is past the target, resets to the targeyt
    (if (or (> _returnvalue 1.0) (< _returnvalue 0.0))
      (set `self.LocationVal` (select `bool` (`self.Opening`) :`true` 1.0))
      (set `self.Opening` false)
      (set `self.Closing` false))
    (bind _returnvalue_2 (`BlueprintEasingLibrary.SineInOut` (`self.LocationVal`)))
    (bind _returnvalue_3 (* _returnvalue_2 600.0))
    ;[1 1 1] Moves both curtains in opposite directions
    (`SceneComponent.K2_SetRelativeLocation` (`self.Curtain1`) (`KismetMathLibrary.MakeVector` (- -380.0 _returnvalue_3) -30.0) false false)
    (`SceneComponent.K2_SetRelativeLocation` (`self.Curtain2`) (`KismetMathLibrary.MakeVector` (+ _returnvalue_3 380.0)) false false)))

(fn `UserConstructionScript`)