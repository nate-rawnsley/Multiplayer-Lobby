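; FontChanger applies the player's saved font style and scale to a given text widget.
; It recovers the original size by dividing the current size by the FontScale in the PreviousSettings save, if present.
; It then multiplies that by the LocalSettings FontScale and picks Roboto or Turtles_Font from the SimpleText flag.
; Without a LocalSettings save it sets Turtles_Font without passing the computed size.
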(fn `ChangeTextAppearance`
  (params (Text :type "TextBlock Object Reference"))
  (locals (TextSize :type "Float (single-precision)") (TextWidget :type "TextBlock Object Reference"))
  (bind (_font_fontobject _font_fontmaterial _font_outlinesettings _font_typefacefontname _font_size) (break `SlateFontInfo` (`TextBlock.Font` Text)))
  (set `local.TextWidget` Text)
  (set `local.TextSize` _font_size)
  (bind _returnvalue (`GameplayStatics.DoesSaveGameExist` "PreviousSettings"))
  (if _returnvalue
    ;[1 1 1] Gets the text's original size by dividing the current size by the previous multiplyer.
    (bind _returnvalue_2 (`GameplayStatics.LoadGameFromSlot` "PreviousSettings"))
    (bind _asplayer_settings (cast `PlayerSettings` _returnvalue_2))
    (set `local.TextSize` (/ (`local.TextSize`) (`PlayerSettings.fontScale` _asplayer_settings))))
  (bind _returnvalue_3 (`GameplayStatics.DoesSaveGameExist` "LocalSettings"))
  (if _returnvalue_3
    (bind _returnvalue_4 (`GameplayStatics.LoadGameFromSlot` "LocalSettings"))
    (bind _asplayer_settings_2 (cast `PlayerSettings` _returnvalue_4))
    ;[1 1 1] Sets the text's font and scale to the saved values.
    (`TextBlock.SetFont` (`local.TextWidget`) (make `SlateFontInfo` (select `bool` (`PlayerSettings.simpleText` _asplayer_settings_2) :`false` "/Game/Turtles_Font.Turtles_Font" :`true` "/Engine/EngineFonts/Roboto.Roboto" :!type "Font Object Reference") null (struct :`OutlineColor` (struct :`A` 1.0)) "None" (* (`PlayerSettings.fontScale` _asplayer_settings_2) (`local.TextSize`))))
    (else
      (`TextBlock.SetFont` (`local.TextWidget`) (make `SlateFontInfo` "/Game/Turtles_Font.Turtles_Font")))))